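; Moving cube actor that shifts vertically once play begins.
; BeginPlay plays a timeline whose track value is added as a local Z offset on each update, so movement accumulates per tick rather than following the curve as position.
; An unconnected second timeline, which sets position from a saved start location plus track times Speed, never runs.
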(event `self.ReceiveBeginPlay`
  (bind (_direction `_新規track_0`) (`Timeline|タイムライン_1`)
    (:`Update`
      (`self.K2_AddActorLocalOffset` (`KismetMathLibrary.MakeVector` 0.0 0.0 `_新規track_0`)))))

(fn `UserConstructionScript`)